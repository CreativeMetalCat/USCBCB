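; Base interactable button whose behavior is driven by a Lua script, with optional key requirement and target actors to trigger.
; BeginPlay starts a Lua machine running Button.lua and passes it the key settings, and Interact forwards the interactor to the script's OnPressed.
; LUA-prefixed functions expose key settings and targets to Lua, while LUAOnSuccess messages each valid target and LUAOnFail is empty.
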(event EventBeginPlay
  (bind _table (CallFunction|RunNewLuaMachine "/Game/Blueprints/Button/LS_Button.LS_Button_C" "LuaCode/Button.lua" "/Game/LuaCode/Button.Button"))
  (bind _output_get (Variables|Default|SetTable _table))
  (Class|LuaComponent|LuaCallTableKey (Variables|Default|GetLua) _output_get "BeginPlay" (Utilities|Array|MakeArray (Class|LuaBlueprintFunctionLibrary|ToLuaValue(Integer) (Variables|Setup|GetKeyID)) (Class|LuaBlueprintFunctionLibrary|ToLuaValue(Boolean) (Variables|Setup|GetNeedsKey)) (Class|LuaBlueprintFunctionLibrary|ToLuaValue(Boolean) (Variables|Setup|GetRemoveKeyOnUse)))))

(event Collision|EventActorBeginOverlap
  (params (OtherActor :type Actor%20Object%20Reference)))

(event EventTick
  (params (DeltaSeconds :type Float%20%28single-precision%29)))

(event EventInteract
  (params (Interactor :type Actor%20Object%20Reference) (InteractedComponent :type Actor%20Component%20Object%20Reference))
  (Class|LuaComponent|LuaCallTableKey (Variables|Default|GetLua) (Variables|Default|GetTable) "OnPressed" (Utilities|Array|MakeArray (Class|LuaBlueprintFunctionLibrary|ToLuaValue(Object) Interactor))))

(fn ConstructionScript)

(fn LUAGetNeedsKey
  (return (Class|LuaBlueprintFunctionLibrary|ToLuaValue(Boolean) (Variables|Setup|GetNeedsKey))))

(fn LUAGetKeyId
  (return (Class|LuaBlueprintFunctionLibrary|ToLuaValue(Integer) (Variables|Setup|GetKeyID))))

(fn LUAGetRemoveKeyonUse
  (return (Class|LuaBlueprintFunctionLibrary|ToLuaValue(Boolean) (Variables|Setup|GetRemoveKeyOnUse))))

(fn LUAonSuccess
  (for _array_element (Variables|Default|GetActors)
    (Utilities|IsValid _array_element
      (:Is%20Valid
        (Class|IInteractions|InteractedbyButton(Message) _array_element self)))))

(fn LUAonFail)

(fn LUAGetAllTargetActors
  (bind _returnvalue (Class|LuaBlueprintFunctionLibrary|LuaCreateTable (Variables|/Script/LuaMachine.LuaComponent|GetLuaState (Variables|Default|GetLua))))
  (LocalVariables|SetArray _returnvalue)
  (for (_array_element _array_index) (Variables|Default|GetActors)
    (Class|LuaBlueprintFunctionLibrary|LuaTableSetField (LocalVariables|GetArray) (Utilities|String|ToString(Integer) _array_index) (Class|LuaBlueprintFunctionLibrary|ToLuaValue(Object) _array_element)))
  (return (LocalVariables|GetArray)))

(fn LUAGetAmountOfTargetActors
  (return (Class|LuaBlueprintFunctionLibrary|ToLuaValue(Integer) (Utilities|Array|Length (Variables|Default|GetActors)))))