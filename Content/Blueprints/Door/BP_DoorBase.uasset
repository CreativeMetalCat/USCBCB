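; Base door actor whose behavior runs in a Lua script, with Blueprint acting as the bridge.
; BeginPlay creates a Lua machine from Door.lua and calls its BeginPlay, while Tick forwards delta time to OnTick.
; Player interaction calls Open, which triggers StartMoving in Lua.
; LUA-prefixed functions expose door state and self to scripts; movement callbacks and Close are empty stubs.
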(event OnLuaError(Lua)
  (params (Message :type String))
  (Development|PrintString Message true true "(R=1.000000,G=0.000000,B=0.000000,A=1.000000)"))

(event EventBeginPlay
  (bind _table (CallFunction|RunNewLuaMachine "/Game/Blueprints/Door/LS_Door.LS_Door_C" "LuaCode/Door.lua" (Variables|Default|GetCode)))
  (bind _output_get (Variables|Default|SetTable _table))
  (Class|LuaComponent|LuaCallTableKey (Variables|Default|GetLua) _output_get "BeginPlay"))

(event Collision|EventActorBeginOverlap
  (params (OtherActor :type Actor%20Object%20Reference)))

(event EventTick
  (params (DeltaSeconds :type Float%20%28single-precision%29))
  (Class|LuaComponent|LuaCallTableKey (Variables|Default|GetLua) (Variables|Default|GetTable) "OnTick" (Utilities|Array|MakeArray (Class|LuaBlueprintFunctionLibrary|ToLuaValue(Float) DeltaSeconds))))

(event EventInteract
  (params (Interactor :type Actor%20Object%20Reference) (InteractedComponent :type Actor%20Component%20Object%20Reference))
  (Utilities|Casting|CastToBP_Player Interactor)
  (CallFunction|Open Interactor))

(fn ConstructionScript)

(fn Open
  (params (Opener :type Actor%20Object%20Reference))
  (Class|LuaComponent|LuaCallTableKey (Variables|Default|GetLua) (Variables|Default|GetTable) "StartMoving" (Utilities|Array|MakeArray (Class|LuaBlueprintFunctionLibrary|ToLuaValue(Object) Opener))))

(fn Close)

(fn LUAUpdateDoorPosition
  (params (Percentage :type Lua%20Value%20Structure)))

(fn LUAonFinishedDoorMovement)

(fn LUAGetIsDoorMoving
  (return ""))

(fn LUAGetIsLocked
  (return (Class|LuaBlueprintFunctionLibrary|ToLuaValue(Boolean) (Variables|Common|GetLocked))))

(fn LUAGetIsOpened
  (return (Class|LuaBlueprintFunctionLibrary|ToLuaValue(Boolean) (Variables|Common|GetOpened))))

(fn LUAGetValue
  (for _array_element (Class|LuaBlueprintFunctionLibrary|LuaTableGetValues (Variables|Default|GetTable))
    _))

(fn LUAGetSelfObject
  (return (Class|LuaBlueprintFunctionLibrary|ToLuaValue(Object) self)))

(fn LUASetIsOpened
  (params (Is :type Lua%20Value%20Structure))
  (Variables|Common|SetOpened (Class|LuaBlueprintFunctionLibrary|ToBoolean(LuaValue) Is)))

(fn LUACanbeInteractedDirectly
  (return (Class|LuaBlueprintFunctionLibrary|ToLuaValue(Boolean) (Variables|Common|GetCanBeInteractedDirectly))))