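; Sliding door Blueprint that extends a parent door class and calls Open when a button interacts with it.
; Opening is delegated to the parent, while the LUAUpdateDoorPosition override slides the lab door mesh along its local Y axis.
; The slide scales a movement distance fetched from a Lua table by the given percentage, with the Opened flag selecting direction and base offset.
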(event EventBeginPlay
  (|CallParentFunction) ; This node is disabled and will not be called.\nDrag off pins to build functionality.
)

(event Collision|EventActorBeginOverlap
  (params (OtherActor :type Actor%20Object%20Reference))
  (|CallParentFunction OtherActor) ; This node is disabled and will not be called.\nDrag off pins to build functionality.
)

(event EventTick
  (params (DeltaSeconds :type Float%20%28single-precision%29))
  (|CallParentFunction DeltaSeconds) ; This node is disabled and will not be called.\nDrag off pins to build functionality.
)

(event EventInteractedbyButton
  (params (Button :type BP%20Button%20Base%20Object%20Reference))
  (CallFunction|Open Button))

(fn ConstructionScript
  (|CallParentFunction))

(fn Open
  (params (Opener :type Actor%20Object%20Reference))
  (|CallParentFunction Opener))

(fn LUAUpdateDoorPosition
  (params (Percentage :type Lua%20Value%20Structure))
  (bind _opened (Variables|Default|GetOpened))
  (|CallParentFunction Percentage)
  (bind _returnvalue (Class|LuaComponent|LuaCallTableKey (Variables|Default|GetLua) (Variables|Default|GetTable) "GetMovementDistance"))
  (Transformation|SetRelativeLocation (Variables|Default|GetSM_LabDoor01) (Math|Vector|MakeVector 0.0 (+ (* (Class|LuaBlueprintFunctionLibrary|ToFloat(LuaValue) _returnvalue) (Class|LuaBlueprintFunctionLibrary|ToFloat(LuaValue) Percentage) (Math|Float|SelectFloat 1.0 -1.0 _opened)) (Math|Float|SelectFloat 1e+02 0.0 _opened)) 0.0) false false))