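; AI controller for SCP-173 that drives the creature through the BT_Peanut behavior tree.
; On BeginPlay it starts the tree and copies the Player reference from the controlled BP_173 pawn into the blackboard.
; Every tick it calls CanMoveMessage on the pawn and writes the result to the CanMove blackboard key, leaving the movement check to the pawn.
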(event EventBeginPlay
  (AI|RunBehaviorTree "/Game/Blueprints/SCPS/173/BT_Peanut.BT_Peanut")
  (bind _asbp_173 (Utilities|Casting|CastToBP_173 (Pawn|GetControlledPawn)))
  (AI|Components|Blackboard|SetValueasObject (Variables|Default|GetBlackboard) (Utilities|Name|MakeLiteralName "Player") (Variables|/Game/Blueprints/SCPS/173/BP_173.BP_173_C|GetPlayer _asbp_173)))

(event EventTick
  (params (DeltaSeconds :type Float%20%28single-precision%29))
  (bind _can (Class|IAI|CanMove(Message) (Pawn|GetControlledPawn)))
  (AI|Components|Blackboard|SetValueasBool (Variables|Default|GetBlackboard) (Utilities|Name|MakeLiteralName "CanMove") _can))

(fn ConstructionScript)