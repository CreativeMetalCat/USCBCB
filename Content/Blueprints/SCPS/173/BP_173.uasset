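; BP_173 is the SCP-173 actor, which may move only while unobserved and plays a horror sting when spotted.
; CanBeSeen combines a recently-rendered check with a visibility trace from above the actor to the player.
; Tick sets WasSeen only when the sting fires, limited by a cooldown timer, and clears it after a short unseen delay.
; CanMove returns true only when both CanBeSeen and WasSeen are false.
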(event Custom|CanSpookAgain
  (Variables|Default|SetCanSpook true))

(event Custom|NoLongerSeen
  (Variables|Default|SetWasSeen false)
  (Utilities|Time|ClearandInvalidateTimerbyHandle (Variables|Default|GetWasSeenTimerHandle)))

(event EventBeginPlay
  (|CallParentFunction) ; This node is disabled and will not be called.\nDrag off pins to build functionality.
)

(event Collision|EventActorBeginOverlap
  (params (OtherActor :type Actor%20Object%20Reference))
  (|CallParentFunction OtherActor) ; This node is disabled and will not be called.\nDrag off pins to build functionality.
)

(event EventTick
  (params (DeltaSeconds :type Float%20%28single-precision%29))
  (|CallParentFunction DeltaSeconds)
  (if (CallFunction|CanbeSeen)
    (if (and (not (Variables|Default|GetWasSeen)) (Variables|Default|GetCanSpook))
      (Audio|PlaySound2D "/Game/SFX/Horror/Horror1.Horror1" 0.5 1.0 0.0 0 0)
      (Utilities|Time|SetTimerbyEvent (delegate Custom|CanSpookAgain) 1e+01)
      (Variables|Default|SetCanSpook false)
      (Variables|Default|SetWasSeen true))
    (elif (not (Utilities|Time|IsValidTimerHandle (Variables|Default|GetWasSeenTimerHandle)))
      (bind _returnvalue (Utilities|Time|SetTimerbyEvent (delegate Custom|NoLongerSeen) 2.0))
      (Variables|Default|SetWasSeenTimerHandle _returnvalue))))

(fn ConstructionScript
  (|CallParentFunction))

(fn CanbeSeen
  (if (Class|Actor|WasRecentlyRendered 0.01)
    (bind (_outhit _returnvalue) (Collision|LineTraceByChannel (+ (Transformation|GetActorLocation) "0, 0,200.000000") (Transformation|GetActorLocation (Variables|Default|GetPlayer)) "TraceTypeQuery1" false 0 "None"))
    (Utilities|Casting|CastToBP_Player (.HitActor (Collision|BreakHitResult _outhit))
      (:then
        (return true))
      (:CastFailed
        _)))
  (return false))

(fn CanMove
  (return (and (not (CallFunction|CanbeSeen)) (not (Variables|Default|GetWasSeen)))))