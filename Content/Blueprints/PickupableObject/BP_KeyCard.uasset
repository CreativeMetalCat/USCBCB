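; BP_KeyCard is a pickupable keycard whose Level variable sets both its item data and its look.
; On Interact by a BP_Player, it fetches the matching KeyCard row from DT_Items and passes it to the player's AddItem.
; If the item is added, it plays a pickup sound and destroys itself.
; The Construction Script swaps both mesh materials by Level, so one Blueprint covers all five keycard tiers.
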(event EventBeginPlay
  (|CallParentFunction) ; This node is disabled and will not be called.\nDrag off pins to build functionality.
)

(event Collision|EventActorBeginOverlap
  (params (OtherActor :type Actor%20Object%20Reference))
  (|CallParentFunction OtherActor) ; This node is disabled and will not be called.\nDrag off pins to build functionality.
)

(event EventTick
  (params (DeltaSeconds :type Float%20%28single-precision%29))
  (|CallParentFunction DeltaSeconds) ; This node is disabled and will not be called.\nDrag off pins to build functionality.
)

(event EventInteract
  (params (Interactor :type Actor%20Object%20Reference) (InteractedComponent :type Actor%20Component%20Object%20Reference))
  (bind _asbp_player (Utilities|Casting|CastToBP_Player Interactor))
  (bind _returnvalue (Utilities|GetDataTableRow "/Game/Blueprints/Inventory/DT_Items.DT_Items" (Utilities|Select :Index (- (Variables|Default|GetLevel) 1) :Option%200 "KeyCard1" :Option%201 "KeyCard2" :Option%202 "KeyCard3" :Option%203 "KeyCard4" :Option%204 "KeyCard5"))
    (:then
      (bind _success (Default|AddItem _asbp_player _returnvalue))
      (if _success
        (Audio|PlaySound2D "/Game/SFX/Interact/PickItem1.PickItem1" 1.0 1.0 0.0 0 0)
        (Actor|DestroyActor)))))

(fn ConstructionScript
  (bind _level (Variables|Default|GetLevel))
  (bind _scp_keycards_level1 (Variables|Default|GetSCP_Keycards_Level1))
  (bind _returnvalue (+ _level -1))
  (|CallParentFunction)
  (Rendering|Material|SetMaterial _scp_keycards_level1 0 (Utilities|Select :Index _returnvalue :Option%200 "/Game/scp-keycards/SCP_Keycards/03_-_Default.03_-_Default" :Option%201 "/Game/scp-keycards/SCP_Keycards/01_-_Default.01_-_Default" :Option%202 "/Game/scp-keycards/SCP_Keycards/08_-_Default.08_-_Default" :Option%203 "/Game/scp-keycards/SCP_Keycards/13_-_Default.13_-_Default" :Option%204 "/Game/scp-keycards/SCP_Keycards/15_-_Default.15_-_Default"))
  (Rendering|Material|SetMaterial _scp_keycards_level1 1 (Utilities|Select :Index _returnvalue :Option%200 "/Game/scp-keycards/SCP_Keycards/07_-_Default.07_-_Default" :Option%201 "/Game/scp-keycards/SCP_Keycards/02_-_Default.02_-_Default" :Option%202 "/Game/scp-keycards/SCP_Keycards/09_-_Default.09_-_Default" :Option%203 "/Game/scp-keycards/SCP_Keycards/14_-_Default.14_-_Default" :Option%204 "/Game/scp-keycards/SCP_Keycards/19_-_Default.19_-_Default")))