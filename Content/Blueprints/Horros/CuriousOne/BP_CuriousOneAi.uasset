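; BP_CuriousOneAi is the AI controller for the Curious One creature, driving it through the BT_CuriousOne behavior tree.
; On BeginPlay it starts the tree and copies the controlled pawn's Player reference into the Blackboard.
; Every tick it queries the pawn through CanMoveMessage and writes the result to the CanMove Blackboard key, so the tree knows whether movement is allowed.
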(event EventBeginPlay
  (AI|RunBehaviorTree "/Game/Blueprints/Horros/CuriousOne/BT_CuriousOne.BT_CuriousOne")
  (bind _asbp_curious_one (Utilities|Casting|CastToBP_CuriousOne (Pawn|GetControlledPawn)))
  (AI|Components|Blackboard|SetValueasObject (Variables|Default|GetBlackboard) (Utilities|Name|MakeLiteralName "Player") (Variables|/Game/Blueprints/Horros/CuriousOne/BP_CuriousOne.BP_CuriousOne_C|GetPlayer _asbp_curious_one)))

(event EventTick
  (params (DeltaSeconds :type Float%20%28single-precision%29))
  (bind _can (Class|IAI|CanMove(Message) (Pawn|GetControlledPawn)))
  (AI|Components|Blackboard|SetValueasBool (Variables|Default|GetBlackboard) (Utilities|Name|MakeLiteralName "CanMove") _can))

(fn ConstructionScript)