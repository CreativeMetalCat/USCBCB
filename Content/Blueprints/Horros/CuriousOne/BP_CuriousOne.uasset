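; BP_CuriousOne is a Weeping Angel-style horror character that freezes while the player watches it.
; CanBeSeen combines recent rendering, line of sight and the player's open eyes, halting movement and playing a cooldown-limited sting.
; Unseen, it kills players inside NeckSnapVolume with line of sight and plays stone-drag audio while moving.
; CanMove also checks a WasSeen flag, cleared by a delayed timer.
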(event Custom|CanSpookAgain
  (Variables|Default|SetCanSpook true))

(event Custom|NoLongerSeen
  (Variables|Default|SetWasSeen false)
  (Utilities|Time|ClearandInvalidateTimerbyHandle (Variables|Default|GetWasSeenTimerHandle)))

(event EventBeginPlay
  (|CallParentFunction) ; This node is disabled and will not be called.\nDrag off pins to build functionality.
)

(event Collision|EventActorBeginOverlap
  (params (OtherActor :type Actor%20Object%20Reference))
  ;[1 0 0] FIX THIS MESS
  (|CallParentFunction OtherActor) ; This node is disabled and will not be called.\nDrag off pins to build functionality.
)

(event EventTick
  (params (DeltaSeconds :type Float%20%28single-precision%29))
  (bind _stonedrag_cue (Variables|Default|GetStoneDrag_Cue))
  (bind _stonedrag_cue_2 (Variables|Default|GetStoneDrag_Cue))
  ;[1 0 0] FIX THIS MESS
  (|CallParentFunction DeltaSeconds)
  (if (CallFunction|CanbeSeen)
    (Audio|Components|Audio|Stop _stonedrag_cue_2)
    (Variables|/Script/Engine.MovementComponent|SetVelocity (Variables|Character|GetCharacterMovement) "0, 0, 0")
    (if (and (not (Variables|Default|GetWasSeen)) (Variables|Default|GetCanSpook))
      (Audio|PlaySound2D "/Game/SFX/Horror/Horror10.Horror10" 0.5 1.0 0.0 0 0)
      (Utilities|Time|SetTimerbyEvent (delegate Custom|CanSpookAgain) 1e+01)
      (Variables|Default|SetCanSpook false)
      (Variables|Default|SetWasSeen true))
    (else
      (if (CallFunction|CanSnap)
        (for _array_element (Collision|GetOverlappingActors (Variables|Default|GetNeckSnapVolume) "/Game/Blueprints/Player/BP_Player.BP_Player_C" :!class /Script/Engine.PrimitiveComponent)
          (bind _asbp_player (Utilities|Casting|CastToBP_Player _array_element))
          (Default|Die _asbp_player)))
      (if (or (Variables|Default|GetStoppingSound) (> (Math|Vector|VectorLength (Transformation|GetVelocity)) 0.0))
        (if (not (Audio|Components|Audio|IsPlaying _stonedrag_cue))
          (Audio|Components|Audio|Play _stonedrag_cue_2 0.0)
          (Variables|Default|SetStoppingSound false))
        (else
          (Audio|Components|Audio|StopDelayed _stonedrag_cue 0.0)
          (Variables|Default|SetStoppingSound true)))
      (if (not (Utilities|Time|IsValidTimerHandle (Variables|Default|GetWasSeenTimerHandle)))
        (bind _returnvalue (Utilities|Time|SetTimerbyEvent (delegate Custom|NoLongerSeen) 3.0))
        (Variables|Default|SetWasSeenTimerHandle _returnvalue)))))

(fn ConstructionScript
  (|CallParentFunction))

(fn CanbeSeen
  (if (Class|Actor|WasRecentlyRendered 0.1)
    (bind (_outhit _returnvalue) (Collision|LineTraceByChannel (+ (Transformation|GetActorLocation) "0, 0,100.000000") (Transformation|GetActorLocation (Variables|Default|GetPlayer)) "TraceTypeQuery1" false (Utilities|Array|MakeArray self) "None"))
    (bind _asbp_player (Utilities|Casting|CastToBP_Player (.HitActor (Collision|BreakHitResult _outhit)))
      (:then
        (if (Variables|/Game/Blueprints/Player/BP_Player.BP_Player_C|GetEyesAreClosed _asbp_player)
          _
          (else
            (return true))))
      (:CastFailed
        _)))
  (return false))

(fn CanSnap
  (bind (_outhit _returnvalue) (Collision|LineTraceByChannel (+ (Transformation|GetActorLocation) "0, 0,100.000000") (Transformation|GetActorLocation (Variables|Default|GetPlayer)) "TraceTypeQuery1" false (Utilities|Array|MakeArray self) "None"))
  (bind _asbp_player (Utilities|Casting|CastToBP_Player (.HitActor (Collision|BreakHitResult _outhit)))
    (:then
      (return true))
    (:CastFailed
      (return false))))

(fn CanMove
  (return (and (not (CallFunction|CanbeSeen)) (not (Variables|Default|GetWasSeen)))))