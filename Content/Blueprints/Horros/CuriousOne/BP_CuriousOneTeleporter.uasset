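; BP_CuriousOneTeleporter is a trigger volume that relocates the Curious One horror when the player walks into it.
; On box overlap by BP_Player, it takes the first BP_CuriousOne in the level and checks its CanBeSeen function.
; If the creature cannot be seen, it moves to the location of a randomly chosen actor from the TargetLocations array.
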(event OnComponentBeginOverlap(Box)
  (params (OverlappedComponent :type Primitive%20Component%20Object%20Reference) (OtherActor :type Actor%20Object%20Reference) (OtherComp :type Primitive%20Component%20Object%20Reference) (OtherBodyIndex :type Integer) (bFromSweep :type Boolean) (SweepResult :type Hit%20Result%20Structure%20%28by%20ref%29))
  (bind _targetlocations (Variables|Default|GetTargetLocations))
  (Utilities|Casting|CastToBP_Player OtherActor)
  (bind _outactors (Actor|GetAllActorsOfClass "/Game/Blueprints/Horros/CuriousOne/BP_CuriousOne.BP_CuriousOne_C"))
  (Utilities|IsValid (Utilities|Array|Get(acopy) _outactors)
    (:Is%20Valid
      (if (not (Default|CanbeSeen (Utilities|Array|Get(acopy) _outactors)))
        (Transformation|SetActorLocation (Utilities|Array|Get(acopy) _outactors) (Transformation|GetActorLocation (Utilities|Array|Get(acopy) _targetlocations (Math|Random|RandomIntegerinRange 0 (- (Utilities|Array|Length _targetlocations) 1)))) false false)))))

(event EventBeginPlay)

(event Collision|EventActorBeginOverlap
  (params (OtherActor :type Actor%20Object%20Reference)))

(event EventTick
  (params (DeltaSeconds :type Float%20%28single-precision%29)))

(fn ConstructionScript)